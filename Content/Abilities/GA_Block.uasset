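; GA_Block is a gameplay ability that puts the owning third-person character into a blocking state.
; On activation it commits, applies the GE_isBlocking effect to the owner and calls the character's Blocking function.
; A wait task ends the ability when the Character.isBlocking tag is removed.
; Ending the ability calls FinishedBlocking on the character and ends the stored wait task.
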(event `self.K2_ActivateAbility`
  (`self.K2_CommitAbility`)
  (`self.BP_ApplyGameplayEffectToOwner` "/Game/Abilities/GE_isBlocking.GE_isBlocking_C")
  (bind _asbp_third_person_character (cast `/Game/ThirdPerson/Blueprints/BP_ThirdPersonCharacter` (`.OwnerActor` (break `GameplayAbilityActorInfo` (`self.GetActorInfo`)))))
  (`/Game/ThirdPerson/Blueprints/BP_ThirdPersonCharacter.Blocking` _asbp_third_person_character)
  (bind _asynctaskproxy (`AbilityTask_WaitGameplayTagRemoved.WaitGameplayTagRemove` (struct :`TagName` "Character.isBlocking") null)
    (:`then`
      (set `self.Wait for tag removal` _asynctaskproxy))
    (:`Removed`
      (`self.K2_EndAbility`))))

(event `self.K2_OnEndAbility`
  (params (bWasCancelled :type Boolean))
  (bind _wait_for_tag_removal (`self.Wait for tag removal`))
  (`/Game/ThirdPerson/Blueprints/BP_ThirdPersonCharacter.FinishedBlocking` (stale `self.K2_ActivateAbility` _asbp_third_person_character))
  (`/Engine/EditorBlueprintResources/StandardMacros.IsValid` _wait_for_tag_removal
    (:`Is Valid`
      (`GameplayTask.EndTask` _wait_for_tag_removal))))